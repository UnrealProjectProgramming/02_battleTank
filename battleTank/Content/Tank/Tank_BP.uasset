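; Tank_BP is the player-controllable tank Blueprint that binds input to movement, camera aiming and firing.
; On BeginPlay it passes the barrel and turret components to the tank and initialises TankMovement with both tracks.
; Movement axes send intents to TankMovement, while aim axes rotate the azimuth gimbal and spring arm at frame-rate-independent speed.
; The Fire action calls Fire, whose logic is not defined in this graph.
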(event `self.ReceiveBeginPlay`
  (`self.SetBarrelReference` (`self.Tank_Barrel`))
  (`self.SetTurretReference` (`self.TankTurret`))
  (`TankMovementComponent.Initialise` (`self.TankMovement`) (`self.Tank_Track_L`) (`self.Tank_Track_R`)))

(event `InputAxis|AimAzimuth`
  (params (AxisValue :type "Float (single-precision)"))
  ;[1 1 1] Aiming
  (`SceneComponent.K2_AddLocalRotation` (`self.Azimuth Gambil`) (`KismetMathLibrary.MakeRotator` 0.0 0.0 (* AxisValue (`GameplayStatics.GetWorldDeltaSeconds`) 100.0)) false false))

(event `InputAxis|Move Forward`
  (params (AxisValue :type "Float (single-precision)"))
  ;[1 1 1] Movment Input Binding
  (`TankMovementComponent.IntendMoveForward` (`self.TankMovement`) AxisValue))

(event `InputAxis|Turn Right`
  (params (AxisValue :type "Float (single-precision)"))
  ;[1 1 1] Movment Input Binding
  (`TankMovementComponent.IntendTurnRight` (`self.TankMovement`) AxisValue))

(event `InputAxis|AimElevation`
  (params (AxisValue :type "Float (single-precision)"))
  ;[1 1 1] Aiming
  (`SceneComponent.K2_AddLocalRotation` (`self.SpringArm`) (`KismetMathLibrary.MakeRotator` 0.0 (* AxisValue (`GameplayStatics.GetWorldDeltaSeconds`) 100.0)) false false))

(event `InputAction|Fire`
  (params (Key :type "Key Structure" :default "AnyKey"))
  ;[1 1 1] Aiming
  (:`Pressed`
    (`self.Fire`)))

(fn `UserConstructionScript`)